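; BP_Food is a grabbable food actor for the baby sim that records where its mesh has been while held.
; GrabComponent's grab and drop events toggle a checking flag, and grabbing also starts the CheckLocation event.
; CheckLocation stores the StaticMesh world location in LastLocation, then repeats through a three-second Delay loop while the flag is set.
; Nothing in this graph reads LastLocation.
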(event `self.ReceiveBeginPlay`)

(event `self.ReceiveTick`
  (params (DeltaSeconds :type "Float (single-precision)")))

(event `self.GrabComponent.OnGrabbed`
  (set `self.isCheckingLocation` true)
  (`self.Check Location`))

(event `self.GrabComponent.OnDropped`
  (set `self.isCheckingLocation` false))

(event `Check Location`
  (if (`self.isCheckingLocation`) :!label _label
    (set `self.Last Location` (`SceneComponent.K2_GetComponentLocation` (`self.StaticMesh`)))
    (`KismetSystemLibrary.Delay` 3.0)
    (goto _label)))

(fn `UserConstructionScript`)