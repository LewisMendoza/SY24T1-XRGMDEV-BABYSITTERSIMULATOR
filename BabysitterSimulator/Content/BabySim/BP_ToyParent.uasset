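; Parent Blueprint for toys in BabySim, handling being picked up and a cooldown that follows.
; PickedUp flags the toy as cooling down, enables actor Tick and turns off physics simulation on the root.
; Tick counts the cooldown down by delta time, then disables itself, clears the flag and resets the timer.
; Physics is not re-enabled in this Blueprint.
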(event `PickedUp`
  (set `self.CoolingDown?` true)
  (`self.SetActorTickEnabled` true)
  (`PrimitiveComponent.SetSimulatePhysics` (`self.Root`) false))

(event `self.ReceiveTick`
  (params (DeltaSeconds :type "Float (single-precision)"))
  (bind _output_get (set `self.CooldownTime` (- (`self.CooldownTime`) (`GameplayStatics.GetWorldDeltaSeconds`))))
  (if (<= _output_get 0.0)
    (`self.SetActorTickEnabled` false)
    (set `self.CoolingDown?` false)
    (set `self.CooldownTime` 10.0)))

(fn `UserConstructionScript`)