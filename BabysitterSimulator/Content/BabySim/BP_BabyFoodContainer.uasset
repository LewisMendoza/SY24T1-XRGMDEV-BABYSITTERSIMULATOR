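; BP_BabyFoodContainer is a baby food container that releases food bits after being struck repeatedly with a BP_BabyFoodHammer.
; Hammer hits on the static mesh pass through a DoOnce, reset after a short Delay as a cooldown, and increment a debug-printed HitCount.
; Once the count has reached its threshold, the next hit calls SpawnFood, which spawns several BP_BabyFoodBits at random points inside the SpawnPoint box and clears the count.
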(event `self.ReceiveBeginPlay`)

(event `self.StaticMesh.OnComponentHit`
  (params (HitComponent :type "PrimitiveComponent Object Reference") (OtherActor :type "Actor Object Reference") (OtherComp :type "PrimitiveComponent Object Reference") (NormalImpulse :type "Vector Structure") (Hit :type "HitResult Structure (by ref)"))
  (bind _hit_count (`self.Hit Count`))
  (cast `/Game/BabySim/BP_BabyFoodHammer` OtherActor)
  (`/Engine/EditorBlueprintResources/StandardMacros.DoOnce` false :!label _label
    (:`Completed`
      (if (< _hit_count 4.0)
        (bind _result (`/Engine/EditorBlueprintResources/StandardMacros.IncrementFloat` _hit_count)
          (:`  `
            (`KismetSystemLibrary.PrintString` (`KismetStringLibrary.Conv_DoubleToString` _result))
            (`KismetSystemLibrary.Delay` 1.0)
            (goto _label :!via `Reset`)))
        (else
          (`self.Spawn Food`)
          (`KismetSystemLibrary.Delay` 1.0)
          (goto _label :!via `Reset`))))))

(event `Spawn Food`
  (bind _spawn_point (`self.Spawn Point`))
  (for _ (range 4)
    (`|SpawnActorFromClass` "/Game/BabySim/BP_BabyFoodBits.BP_BabyFoodBits_C" (`KismetMathLibrary.MakeTransform` (`KismetMathLibrary.RandomPointInBoundingBox` (`SceneComponent.K2_GetComponentLocation` _spawn_point) (`BoxComponent.BoxExtent` _spawn_point))) "Undefined" "MultiplyWithRoot" null null)
    (set `self.Hit Count` 0.0)))

(fn `UserConstructionScript`)