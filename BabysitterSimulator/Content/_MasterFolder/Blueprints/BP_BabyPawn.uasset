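; BP_BabyPawn is a baby pawn that wanders on its own and can be grabbed and dropped.
; From BeginPlay, FreeRoam runs AI moves to random reachable points nearby, chaining on success while not ragdolled.
; GrabComponentSnap's grab and drop events both toggle ragdoll mode, switching physics simulation on the baby mesh.
; Nothing restarts roaming when ragdoll ends or a move fails.
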(event `self.ReceiveBeginPlay`
  (`self.FreeRoam`))

(event `FreeRoam`
  (`|AIMoveTo` self (`NavigationSystemV1.K2_GetRandomReachablePointInRadius` (`self.K2_GetActorLocation`) 100.0 null null) null
    (:`OnSuccess`
      (if (not (`self.RagdollMode`))
        (`self.FreeRoam`)))))

(event `self.GrabComponentSnap.OnGrabbed`
  (`self.SetRagdollMode`))

(event `self.GrabComponentSnap.OnDropped`
  (`self.SetRagdollMode`))

(fn `SetRagdollMode`
  (bind _babymesh (`self.BabyMesh`))
  (if (`self.RagdollMode`)
    (`PrimitiveComponent.SetSimulatePhysics` _babymesh false)
    (set `self.RagdollMode` false)
    (else
      (`PrimitiveComponent.SetSimulatePhysics` _babymesh true)
      (set `self.RagdollMode` true))))

(fn `UserConstructionScript`)