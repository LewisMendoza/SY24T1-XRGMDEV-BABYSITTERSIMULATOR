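; BP_BabyCharacterr is an AI baby character that wanders at random and can be grabbed.
; FreeRoam moves it to random reachable nearby points, pausing randomly after each successful move and repeating unless ragdolled.
; GrabComponent's grab and drop events both toggle ragdoll through SetRagdollMode, which switches mesh physics, then resets mesh rotation and resumes roaming on exit.
; BabyHappiness drops every tick and wraps back to full at zero.
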(event `self.ReceiveBeginPlay`
  (`self.Free Roam`)
  (set `self.BabyState` "NewEnumerator0"))

(event `Free Roam`
  (`|AIMoveTo` self (`NavigationSystemV1.K2_GetRandomReachablePointInRadius` (`self.K2_GetActorLocation`) 500.0 null null) null
    (:`OnSuccess`
      (`KismetSystemLibrary.Delay` (`KismetMathLibrary.RandomFloatInRange` 0.0 6.0))
      (if (not (`self.RagdollMode`))
        (`self.Free Roam`)))))

(event `self.ReceiveTick`
  (params (DeltaSeconds :type "Float (single-precision)"))
  (bind _result (`/Engine/EditorBlueprintResources/StandardMacros.DecrementFloat` (`self.BabyHappiness`))
    (:`  `
      (bind _output_get (set `self.BabyHappiness` _result))
      (if (<= _output_get 0.0)
        (set `self.BabyHappiness` 100.0)))))

(event `self.GrabComponent.OnGrabbed`
  (`self.SetRagdollMode`))

(event `self.GrabComponent.OnDropped`
  (`self.SetRagdollMode`))

(fn `SetRagdollMode`
  (bind _mesh (`self.Mesh`))
  (if (`self.RagdollMode`)
    (`PrimitiveComponent.SetSimulatePhysics` _mesh false)
    (set `self.RagdollMode` false)
    (`SceneComponent.K2_SetRelativeRotation` (`self.Mesh`) (struct :`Yaw` -90.0) false false)
    (`self.Free Roam`)
    (else
      (`PrimitiveComponent.SetSimulatePhysics` _mesh true)
      (set `self.RagdollMode` true))))

(fn `UserConstructionScript`)