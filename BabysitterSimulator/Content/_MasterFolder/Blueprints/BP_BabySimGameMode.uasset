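; Game mode for a baby simulation that runs a countdown and rates the player by the baby's state.
; Tick decrements Timer and, once it runs out, maps BabyReference's BabyState to a one-to-three star Score.
; The score is printed on screen every frame from then on, as the timer is never reset.
; A RestartLevel event reopens VRTemplateMap.
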(event `self.ReceiveTick`
  (params (DeltaSeconds :type "Float (single-precision)"))
  (bind _output_get (set `self.Timer` (- (`self.Timer`) DeltaSeconds)))
  (if (<= _output_get 0.0)
    (switch `/Game/_MasterFolder/Data/E_BabyStateEnum` (`/Game/_MasterFolder/Blueprints/BP_BabyCharacterr.BabyState` (`self.Baby Reference`))
      (:`NewEnumerator0`
        (set `self.Score` "2 Star"))
      (:`NewEnumerator1`
        (set `self.Score` "3 Star"))
      (:`NewEnumerator2`
        (set `self.Score` "1 Star")))
    (`KismetSystemLibrary.PrintString` (`self.Score`) true false (struct :`G` 1.0 :`B` 0.240991 :`A` 1.0) 0.0)))

(event `Restart Level`
  (`GameplayStatics.OpenLevel` "VRTemplateMap"))

(fn `UserConstructionScript`)